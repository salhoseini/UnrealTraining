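; Base gadget actor that bobs up and down and spins in place.
; BeginPlay records the starting Z, and Tick calls Play on a timeline every frame.
; Each timeline update offsets Z from that start by the scaled bob track and advances yaw by spin speed times Tick's delta seconds.
; The overlap event and construction script are empty.
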(event EventBeginPlay
  (Variables|Default|SetStartingZPosition (.z (Transformation|GetActorLocation))))

(event Collision|EventActorBeginOverlap
  (params (OtherActor :type Actor%20Object%20Reference)))

(event EventTick
  (params (DeltaSeconds :type Float%20%28single-precision%29))
  (bind _returnvalue (Transformation|GetActorLocation))
  (bind _returnvalue_2 (Transformation|GetActorRotation))
  (bind _bobupanddowntrack (Timeline|Timeline Play)
    (:Update
      (Transformation|SetActorLocation (Math|Vector|MakeVector (.x _returnvalue) (.y _returnvalue) (+ (* _bobupanddowntrack (Variables|Default|GetBobOffset)) (Variables|Default|GetStartingZPosition))) false false)
      (Transformation|SetActorRotation (Math|Rotator|MakeRotator (.roll _returnvalue_2) (.pitch _returnvalue_2) (+ (* DeltaSeconds (Variables|Default|GetSpinAnglePerSecond)) (.yaw _returnvalue_2)))))))

(fn ConstructionScript)